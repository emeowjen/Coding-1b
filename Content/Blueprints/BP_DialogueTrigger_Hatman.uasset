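; BP_DialogueTrigger_Hatman is a dialogue trigger that shows the Hatman's lines in a dialogue widget.
; Its sphere collision adds and removes a W_Prompt widget, created at BeginPlay, as the player character enters and leaves.
; Each Talk call increments an index into DialogueHatMan, creating W_Dialogue if needed and setting its text.
; Once the index passes the last line, the dialogue widget is removed; nothing here resets the index.
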(event OnComponentBeginOverlap(SphereCollision)
  (params (OverlappedComponent :type Primitive%20Component%20Object%20Reference) (OtherActor :type Actor%20Object%20Reference) (OtherComp :type Primitive%20Component%20Object%20Reference) (OtherBodyIndex :type Integer) (bFromSweep :type Boolean) (SweepResult :type Hit%20Result%20Structure%20%28by%20ref%29))
  (if (== OtherActor (Game|GetPlayerCharacter 0))
    (UserInterface|Viewport|AddtoViewport (Variables|Default|GetInteractWidget) 0)))

(event OnComponentEndOverlap(SphereCollision)
  (params (OverlappedComponent :type Primitive%20Component%20Object%20Reference) (OtherActor :type Actor%20Object%20Reference) (OtherComp :type Primitive%20Component%20Object%20Reference) (OtherBodyIndex :type Integer))
  (if (== (Game|GetPlayerCharacter 0) OtherActor)
    (Widget|RemovefromParent (Variables|Default|GetInteractWidget))))

(event EventTick
  (params (DeltaSeconds :type Float%20%28single-precision%29)))

(event EventBeginPlay
  (bind _returnvalue (UserInterface|CreateWidget "/Game/Widgets/W_Prompt.W_Prompt_C"))
  (Variables|Default|SetInteractWidget _returnvalue))

(event EventTalk
  (Math|Integer|IncrementInt (Variables|Default|GetTalkIndex)
    (:%20%20
      (if (< (Variables|Default|GetTalkIndex) (Utilities|Array|Length (Variables|Default|GetDialogue%28HatMan%29)))
        (Variables|Default|GetUI
          (:then
            _)
          (:else
            (bind _returnvalue (UserInterface|CreateWidget "/Game/Widgets/W_Dialogue.W_Dialogue_C" (Game|GetPlayerController 0)))
            (bind _output_get (Variables|Default|SetUI _returnvalue))
            (UserInterface|Viewport|AddtoViewport _output_get 0)))
        (Rendering|Components|TextRender|SetText (Variables|/Game/Widgets/W_Dialogue.W_Dialogue_C|GetDialogueText (Variables|Default|GetUI)) (Utilities|Array|Get(acopy) (Variables|Default|GetDialogue%28HatMan%29) (Variables|Default|GetTalkIndex)))
        (else
          (Widget|RemovefromParent (Variables|Default|GetUI)))))))

(fn ConstructionScript)