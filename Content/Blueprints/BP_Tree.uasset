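; Tree actor that grows in random steps after play begins.
; BeginPlay runs a looping Do N gate with a random limit of a few passes, each waiting a random Delay before calling Grow.
; Grow adds a random increment to the SMTree mesh's relative scale.
; A branch on the Do N counter equalling zero would set physics-only collision and print a debug message; otherwise execution loops back into the gate.
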(event Custom|Grow
  (bind _sm_tree (Variables|Default|GetSM_Tree))
  (Transformation|SetRelativeScale3D _sm_tree (+ (Variables|/Script/Engine.SceneComponent|GetRelativeScale3D _sm_tree) (Math|Random|RandomFloatinRange 0.2 0.4))))

(event Collision|EventActorBeginOverlap
  (params (OtherActor :type Actor%20Object%20Reference)))

(event EventTick
  (params (DeltaSeconds :type Float%20%28single-precision%29)))

(event EventBeginPlay
  (bind _counter (Utilities|FlowControl|DoN (Math|Random|RandomIntegerinRange 1 5) :!label _label)
    (:Exit
      (Utilities|FlowControl|Delay (Math|Random|RandomFloatinRange 3.0 5.0))
      (CallFunction|Grow)
      (if (== _counter 0)
        (Collision|SetCollisionEnabled (Variables|Default|GetSM_Tree) "PhysicsOnly")
        (Development|PrintText "Collision enabled")
        (else
          (goto _label))))))

(fn ConstructionScript)