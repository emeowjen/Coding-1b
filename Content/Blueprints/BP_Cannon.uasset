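; BP_Cannon is an actor that fires cannonballs automatically and endlessly from the start of play.
; BeginPlay runs a short Delay loop that repeatedly calls the FireCannon event.
; FireCannon prints a debug message, spawns a BP_CanonBall at the SpawnPoint transform, then launches its Cube component along the SpawnPoint forward vector using a mass-independent AddForce.
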(event Custom|FireCannon
  (Development|PrintText "Canon is firing!")
  (bind _returnvalue (Game|SpawnActorfromClass "/Game/Blueprints/BP_CanonBall.BP_CanonBall_C" (Transformation|GetWorldTransform (Variables|Default|GetSpawnPoint)) "Undefined" "MultiplyWithRoot" 0 0))
  (Physics|AddForce (Variables|/Game/Blueprints/BP_CanonBall.BP_CanonBall_C|GetCube _returnvalue) (* (Math|Vector|GetForwardVector (Variables|Default|GetSpawnPoint)) 1e+05) "None" true))

(event EventBeginPlay
  (Utilities|FlowControl|Delay 0.2 :!label _label)
  (CallFunction|FireCannon)
  (goto _label))

(fn ConstructionScript)