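; BP_Door is a locked door actor that the third-person player character opens by spending a key.
; Overlapping its box prints a hint, then checks the character's TotalKeys count.
; With a key, it decrements the count, plays a success sound and destroys the door mesh and overlap box, opening it permanently.
; Without one, it plays a failure sound and prints a refusal message.
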(event EventBeginPlay)

(event EventTick
  (params (DeltaSeconds :type Float%20%28single-precision%29)))

(event Collision|EventActorBeginOverlap
  (params (OtherActor :type Actor%20Object%20Reference))
  (bind _asbp_third_person_character (Utilities|Casting|CastToBP_ThirdPersonCharacter OtherActor))
  (Development|PrintText "I wish I could go through this door...")
  (if (> (Variables|/Game/ThirdPerson/Blueprints/BP_ThirdPersonCharacter.BP_ThirdPersonCharacter_C|GetTotalKeys _asbp_third_person_character) 0) ; if they have a key, open the door!\nelse, laugh at them lol
    (Math|Integer|DecrementInt (Variables|/Game/ThirdPerson/Blueprints/BP_ThirdPersonCharacter.BP_ThirdPersonCharacter_C|GetTotalKeys _asbp_third_person_character)
      (:%20%20
        (Audio|PlaySound2D "/Engine/EditorSounds/Notifications/CompileSuccess.CompileSuccess" 1.0 1.0 0.0 0 0)
        (Components|DestroyComponent (Variables|Default|GetSM_Bld_Door_01))
        (Components|DestroyComponent (Variables|Default|GetOverlapBox))))
    (else
      (Audio|PlaySound2D "/Engine/EditorSounds/Notifications/CompileFailed.CompileFailed" 1.0 1.0 0.0 0 0)
      (Development|PrintText "You don't qualify to enter."))))

(fn ConstructionScript)