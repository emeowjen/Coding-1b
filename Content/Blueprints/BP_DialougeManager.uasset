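; BP_DialougeManager is a dialogue manager that shows lines from a Dialogue array one at a time.
; It creates a W_Dialogue widget on BeginPlay and reuses it for each DisplayNextLine call.
; Each call prints the current line, shows it in the widget for five seconds, and advances the index without waiting.
; Past the last line, it restarts if ShouldRepeatText is set, otherwise does nothing.
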(event Custom|DisplayNextLine
  (bind _dialougewidget (Variables|Default|GetDialougeWidget))
  (if (>= (Variables|Default|GetIndex) (Utilities|Array|Length (Variables|Default|GetDialogue)))
    (if (Variables|Default|GetShouldRepeatText)
      (Variables|Default|SetIndex 0)
      (Development|PrintText (Utilities|Array|Get(acopy) (Variables|Default|GetDialogue) (Variables|Default|GetIndex)) true true "(R=1.000000,G=0.962527,B=0.952092,A=1.000000)" 5.0 :!label _label)
      (Rendering|Components|TextRender|SetText (Variables|/Game/Widgets/W_Dialogue.W_Dialogue_C|GetDialogueText (Variables|Default|GetDialougeWidget)) (Utilities|Array|Get(acopy) (Variables|Default|GetDialogue) (Variables|Default|GetIndex)))
      (Utilities|FlowControl|Sequence
        (:then_0
          (UserInterface|Viewport|AddtoViewport _dialougewidget 0)
          (Utilities|FlowControl|Delay 5.0)
          (Widget|RemovefromParent _dialougewidget))
        (:then_1
          (Math|Integer|IncrementInt (Variables|Default|GetIndex)) ; Increment Int\nadd 1 to index
        )))
    (else
      (goto _label))))

(event EventBeginPlay
  (bind _returnvalue (UserInterface|CreateWidget "/Game/Widgets/W_Dialogue.W_Dialogue_C"))
  (Variables|Default|SetDialougeWidget _returnvalue))

(fn ConstructionScript)