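; BP_LoopsAndLists is a demo actor of loop techniques that randomly rotates BP_CherryTree actors in the level.
; On BeginPlay, a Delay-driven endless loop repeatedly calls LoopArrayOverTime, which shuffles the trees and staggers yaw changes using an index and short delays.
; A while loop also prints a countdown in cycling colors.
; ChangeTreesForEach rotates all trees at once but is not called in this graph.
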(event Custom|Simple%20Loop
  ;[0.02109 0.15 0.06663 0.5] Rotating Tree Loop
  (Development|PrintText "Inside Simple Loop, waiting 3 seconds." :!label _label)
  (CallFunction|LoopArrayOverTime)
  (Utilities|FlowControl|Delay 3.0)
  (goto _label))

(event Custom|WhileLoop%20Function
  (bind _colors (Variables|Default|GetColors))
  ;[0.02109 0.15 0.06663 0.5] Rotating Tree Loop
  (while (> (Variables|Default|GetWhileCounter) 0) ; If condition is true, \nkeep looping
    (Development|PrintText (Utilities|Text|FormatText "This is loop {count}. Ran after {seconds} seconds." (Variables|Default|GetWhileCounter) (Utilities|Text|ToText(Float) (Utilities|Time|GetRealTimeSeconds) "HalfToEven" false true 1 324 3)) true true (Utilities|Array|Get(acopy) _colors (Math|Integer|%(Integer) (Variables|Default|GetWhileCounter) (Utilities|Array|Length _colors))) 2e+01)
    (Math|Integer|DecrementInt (Variables|Default|GetWhileCounter))))

(event Custom|ChangeTreesForEach
  ;[0.02109 0.15 0.06663 0.5] Rotating Tree Loop
  (bind _outactors (Actor|GetAllActorsOfClass "/Game/Blueprints/BP_CherryTree.BP_CherryTree_C"))
  (for _array_element _outactors
    (Transformation|SetActorRelativeRotation _array_element (Math|Rotator|MakeRotator 0.0 0.0 (Math|Random|RandomFloatinRange 0.0 3.7e+02))))
  (Development|PrintText "Trees have been rotated!"))

(event Custom|LoopArrayOverTime
  ;[0.02109 0.15 0.06663 0.5] Rotating Tree Loop
  (bind _outactors (Actor|GetAllActorsOfClass "/Game/Blueprints/BP_CherryTree.BP_CherryTree_C"))
  (Utilities|Array|Shuffle _outactors)
  (if (< (Variables|Default|GetOverTimeIndex) (Utilities|Array|Length _outactors)) :!label _label
    (Transformation|SetActorRelativeRotation (Utilities|Array|Get(acopy) _outactors (Variables|Default|GetOverTimeIndex)) (Math|Rotator|MakeRotator 0.0 0.0 (Math|Random|RandomFloatinRange 0.0 3.7e+02)))
    (Math|Integer|IncrementInt (Variables|Default|GetOverTimeIndex)
      (:%20%20
        (Utilities|FlowControl|Delay 0.2)
        (goto _label)))
    (else
      (Variables|Default|SetOverTimeIndex 0))))

(event EventBeginPlay
  ;[0.02109 0.15 0.06663 0.5] Rotating Tree Loop
  (Development|PrintText "Loops and Lists is starting!" true true "(R=0.000000,G=0.660000,B=1.000000,A=1.000000)" 3.0)
  (CallFunction|SimpleLoop)
  (CallFunction|WhileLoopFunction))

(event Collision|EventActorBeginOverlap
  (params (OtherActor :type Actor%20Object%20Reference)))

(event EventTick
  (params (DeltaSeconds :type Float%20%28single-precision%29)))

(fn ConstructionScript)