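; BP_KillerHat is an overlap-triggered hat actor that shows dialogue and teleports the player to a fixed location.
; Any overlap creates a W_Dialogue widget showing the DialogueHatMan line at TalkIndex, before checking what overlapped.
; If the overlapping actor is BP_ThirdPersonCharacter, the hat waits briefly, destroys itself, then teleports the character.
; The widget is never removed here, and TalkIndex never changes.
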(event EventBeginPlay)

(event Collision|EventActorBeginOverlap
  (params (OtherActor :type Actor%20Object%20Reference))
  (bind _returnvalue (UserInterface|CreateWidget "/Game/Widgets/W_Dialogue.W_Dialogue_C"))
  (bind _output_get (Variables|Default|SetUI _returnvalue))
  (UserInterface|Viewport|AddtoViewport _output_get 0)
  (Rendering|Components|TextRender|SetText (Variables|/Game/Widgets/W_Dialogue.W_Dialogue_C|GetDialogueText (Variables|Default|GetUI)) (Utilities|Array|Get(acopy) (Variables|Default|GetDialogue%28Hat%20Man%29) (Variables|Default|GetTalk%20Index)))
  (bind _asbp_third_person_character (Utilities|Casting|CastToBP_ThirdPersonCharacter OtherActor)) ; Was it the player that hit us?
  (if true
    (bind _output_get_2 (Variables|Default|SetAs%20BP%20Third%20Person%20Character _asbp_third_person_character))
    (Utilities|FlowControl|Delay 0.5)
    (Actor|DestroyActor)
    (Transformation|Teleport _output_get_2 "-1270.000000,1270.000000,2142.000000" "0, 0, 0")))

(event EventTick
  (params (DeltaSeconds :type Float%20%28single-precision%29)))

(fn ConstructionScript)