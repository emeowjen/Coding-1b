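; BP_Basket is an overlap-triggered hat drop-off that responds when the third-person character enters holding a BP_TrueHat.
; It decrements the character's hat count, calls the hat's DropMessage, plays a cheer and creates a W_Dialogue widget showing the DialogueHatMan line at TalkIndex.
; The branch condition is hardcoded true, so the "no hats" print never runs; failed casts simply stop.
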(event EventBeginPlay)

(event EventTick
  (params (DeltaSeconds :type Float%20%28single-precision%29)))

(event Collision|EventActorBeginOverlap
  (params (OtherActor :type Actor%20Object%20Reference))
  (bind _asbp_third_person_character (Utilities|Casting|CastToBP_ThirdPersonCharacter OtherActor))
  (bind _asbp_true_hat (Utilities|Casting|CastToBP_TrueHat (Variables|/Game/ThirdPerson/Blueprints/BP_ThirdPersonCharacter.BP_ThirdPersonCharacter_C|GetHeldItem _asbp_third_person_character)))
  (if true
    (Math|Integer|DecrementInt (Variables|/Game/ThirdPerson/Blueprints/BP_ThirdPersonCharacter.BP_ThirdPersonCharacter_C|GetTotalHatCount _asbp_third_person_character)
      (:%20%20
        (Class|BPIItem|Drop(Message) _asbp_true_hat)
        (Audio|PlaySound2D "/Game/Audio/428156__higgs01__yay.428156__higgs01__yay" 1.0 1.0 0.0 0 0)
        (bind _returnvalue (UserInterface|CreateWidget "/Game/Widgets/W_Dialogue.W_Dialogue_C"))
        (bind _output_get (Variables|Default|SetUI _returnvalue))
        (UserInterface|Viewport|AddtoViewport _output_get 0)
        (Rendering|Components|TextRender|SetText (Variables|/Game/Widgets/W_Dialogue.W_Dialogue_C|GetDialogueText (Variables|Default|GetUI)) (Utilities|Array|Get(acopy) (Variables|Default|GetDialogue%28Hat%20Man%29) (Variables|Default|GetTalk%20Index)))))
    (else
      (Development|PrintText "I don't have any hats to give..." true true "(R=1.000000,G=1.000000,B=1.000000,A=1.000000)"))))

(fn ConstructionScript)