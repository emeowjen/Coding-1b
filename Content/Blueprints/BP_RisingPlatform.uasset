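; BP_RisingPlatform is an actor that moves back and forth continuously from its placed location, starting at BeginPlay.
; It caches the start location, then a timeline track supplies an offset that is added to it each update, setting the position without sweep.
; When the timeline finishes, its direction selects MoveToStart or MoveToEnd, so it reverses or replays in an endless ping-pong loop.
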(event Custom|Move%20to%20start
  (bind (_direction _newtrack_0) (Timeline|Timeline ReverseFromEnd)
    (:Update
      (Transformation|SetActorLocation (+ (Variables|Default|GetStart) _newtrack_0) false false))
    (:Finished
      (switch Utilities|FlowControl|Switch|SwitchonETimelineDirection _direction
        (:Forward
          (CallFunction|MovetoStart))
        (:Backward
          (CallFunction|MovetoEnd))))))

(event Custom|Move%20to%20end
  (bind (_direction _newtrack_0) (Timeline|Timeline PlayFromStart)
    (:Update
      (Transformation|SetActorLocation (+ (Variables|Default|GetStart) _newtrack_0) false false))
    (:Finished
      (switch Utilities|FlowControl|Switch|SwitchonETimelineDirection _direction
        (:Forward
          (CallFunction|MovetoStart))
        (:Backward
          (CallFunction|MovetoEnd))))))

(event EventBeginPlay
  (Variables|Default|SetStart (Transformation|GetActorLocation))
  (CallFunction|MovetoEnd))

(fn ConstructionScript)