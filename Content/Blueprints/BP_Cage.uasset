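; BP_Cage is a locked cage that the third-person character opens by spending a cage key.
; On actor overlap it casts to BP_ThirdPersonCharacter and checks TotalCageKeys.
; With a key available, it decrements the count, destroys the box cage and overlap box components, then performs a component attach using relative transform rules.
; Without a key, it prints a locked message.
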(event Collision|EventActorBeginOverlap
  (params (OtherActor :type Actor%20Object%20Reference))
  (bind _asbp_third_person_character (Utilities|Casting|CastToBP_ThirdPersonCharacter OtherActor))
  (if (> (Variables|/Game/ThirdPerson/Blueprints/BP_ThirdPersonCharacter.BP_ThirdPersonCharacter_C|GetTotalCageKeys _asbp_third_person_character) 0)
    (Math|Integer|DecrementInt (Variables|/Game/ThirdPerson/Blueprints/BP_ThirdPersonCharacter.BP_ThirdPersonCharacter_C|GetTotalCageKeys _asbp_third_person_character)
      (:%20%20
        (Components|DestroyComponent (Variables|Default|Getbox_cage))
        (Components|DestroyComponent (Variables|Default|GetOverlapBox))
        (Transformation|AttachComponentToComponent 0 "None" "KeepRelative" "KeepRelative" "KeepRelative" true)))
    (else
      (Development|PrintText "This cage is locked."))))

(fn ConstructionScript)