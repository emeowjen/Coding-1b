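; BP_TrueHat is a pickup actor for the hat the Hatman wants, worn on the player's head.
; On overlap with BP_ThirdPersonCharacter it stores the player, passes itself to TryToPickUpItem and destroys its RotatingMovement component to stop spinning.
; Its Pickup event attaches it to the "head" socket of the player's mesh, while Drop destroys the actor.
; Each event prints a message.
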(event Collision|EventActorBeginOverlap
  (params (OtherActor :type Actor%20Object%20Reference))
  (Development|PrintText "I think this is the hat the Hatman wanted!")
  (bind _asbp_third_person_character (Utilities|Casting|CastToBP_ThirdPersonCharacter OtherActor))
  (Variables|Default|SetPlayer _asbp_third_person_character)
  (Default|TrytoPickUpItem _asbp_third_person_character self)
  (Components|DestroyComponent (Variables|Default|GetRotatingMovement)))

(event EventPickup
  (Development|PrintText "Let me pick up this hat.")
  (Transformation|AttachComponentToComponent (Variables|/Script/Engine.Character|GetMesh (Variables|Default|GetPlayer)) "head" "SnapToTarget" "KeepWorld" "KeepRelative" true))

(event EventDrop
  (Development|PrintText "The hat is being dropped.")
  (Actor|DestroyActor))

(fn ConstructionScript)