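; BP_CageKey is a rotating cage key pickup that the third-person character collects by overlapping it.
; On overlap it increments the character's key count, offers itself through TryToPickUpItem, then destroys its collision sphere and rotating movement.
; Its Pickup event attaches the key to the character mesh's right-hand grip socket, Drop destroys the actor, and PrimaryAction is empty.
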(event EventDrop
  (Development|PrintText "The key has been dropped.")
  (Actor|DestroyActor))

(event EventPrimaryAction)

(event Collision|EventActorBeginOverlap
  (params (OtherActor :type Actor%20Object%20Reference))
  (bind _asbp_third_person_character (Utilities|Casting|CastToBP_ThirdPersonCharacter OtherActor))
  (Default|GetTotalCageKeys _asbp_third_person_character (Variables|Default|GetCageKeyAmount))
  (Math|Integer|IncrementInt (Variables|/Game/ThirdPerson/Blueprints/BP_ThirdPersonCharacter.BP_ThirdPersonCharacter_C|GetTotalCageKeyCount _asbp_third_person_character)
    (:%20%20
      (Variables|Default|SetPlayer _asbp_third_person_character)
      (Default|TrytoPickUpItem _asbp_third_person_character self)
      (Components|DestroyComponent (Variables|Default|GetSphereCollision))
      (Components|DestroyComponent (Variables|Default|GetRotatingMovement)))))

(event EventPickup
  (Development|PrintText "Let me pick up this key.")
  (Transformation|AttachComponentToComponent (Variables|/Script/Engine.Character|GetMesh (Variables|Default|GetPlayer)) "handgrip_r" "SnapToTarget" "SnapToTarget" "KeepRelative" true))

(fn ConstructionScript)