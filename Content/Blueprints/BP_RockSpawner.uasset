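; BP_RockSpawner is a pickup item, described in its debug text as a rock planter, that the third-person character can carry and use.
; On overlap it caches the character and calls its TryToPickUpItem.
; Pickup, PrimaryAction and Drop events respectively attach it to the right-hand grip socket, spawn an actor at its transform, and destroy it.
; Despite the rock naming, the spawned class is BP_Tree.
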(event Collision|EventActorBeginOverlap
  (params (OtherActor :type Actor%20Object%20Reference))
  (bind _asbp_third_person_character (Utilities|Casting|CastToBP_ThirdPersonCharacter OtherActor))
  (Variables|Default|SetPlayer _asbp_third_person_character)
  (Default|TrytoPickUpItem _asbp_third_person_character self))

(event EventPickup
  (Development|PrintText "The rock planter is getting picked up")
  (Transformation|AttachComponentToComponent (Variables|/Script/Engine.Character|GetMesh (Variables|Default|GetPlayer)) "handgrip_r" "SnapToTarget" "SnapToTarget" "KeepRelative" true))

(event EventPrimaryAction
  (Development|PrintText "Le'ts plant some rocks!")
  (Game|SpawnActorfromClass "/Game/Blueprints/BP_Tree.BP_Tree_C" (Transformation|GetActorTransform) "Undefined" "MultiplyWithRoot" 0 0))

(event EventDrop
  (Development|PrintText "The rock planter is getting dropped.")
  (Actor|DestroyActor))

(fn ConstructionScript)