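; BP_CringeHat is a hat actor that reacts to being touched, apparently as a wrong find in a hat-related dialogue exchange.
; On any actor overlap it destroys itself, prints a doubtful "I don't think this is it..." message and adds a W_Dialogue widget to the viewport.
; The widget shows the DialogueHatMan line at TalkIndex, an index this graph never advances.
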(event EventBeginPlay)

(event Collision|EventActorBeginOverlap
  (params (OtherActor :type Actor%20Object%20Reference))
  (Actor|DestroyActor)
  (Development|PrintText "I don't think this is it..." true true "(R=1.000000,G=1.000000,B=1.000000,A=1.000000)")
  (bind _returnvalue (UserInterface|CreateWidget "/Game/Widgets/W_Dialogue.W_Dialogue_C"))
  (bind _output_get (Variables|Default|SetUI _returnvalue))
  (UserInterface|Viewport|AddtoViewport _output_get 0)
  (Rendering|Components|TextRender|SetText (Variables|/Game/Widgets/W_Dialogue.W_Dialogue_C|GetDialogueText (Variables|Default|GetUI)) (Utilities|Array|Get(acopy) (Variables|Default|GetDialogue%28Hat%20Man%29) (Variables|Default|GetTalk%20Index))))

(event EventTick
  (params (DeltaSeconds :type Float%20%28single-precision%29)))

(fn ConstructionScript)