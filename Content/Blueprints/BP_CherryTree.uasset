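; Cherry tree actor that grows its mesh in random increments after play begins.
; BeginPlay loops through a random-limit DoN gate, waiting a few seconds before each Grow call adds to the mesh's relative scale.
; A branch would end the loop by switching the mesh to physics-only collision, but its random roll can never match, so only the DoN limit stops growth.
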(event Custom|Grow
  (bind _sm_generic_tree_01 (Variables|Default|GetSM_Generic_Tree_01))
  (Transformation|SetRelativeScale3D _sm_generic_tree_01 (+ (Variables|/Script/Engine.SceneComponent|GetRelativeScale3D _sm_generic_tree_01) (Math|Random|RandomFloatinRange 0.2 0.4))))

(event EventBeginPlay
  (bind _returnvalue (Math|Random|RandomIntegerinRange 1 5))
  (Utilities|FlowControl|DoN _returnvalue :!label _label
    (:Exit
      (Utilities|FlowControl|Delay (Math|Random|RandomFloatinRange 3.0 5.0))
      (CallFunction|Grow)
      (if (== _returnvalue 0)
        (Collision|SetCollisionEnabled (Variables|Default|GetSM_Generic_Tree_01) "PhysicsOnly")
        (Development|PrintText "Collision enabled")
        (else
          (goto _label))))))

(event Collision|EventActorBeginOverlap
  (params (OtherActor :type Actor%20Object%20Reference)))

(event EventTick
  (params (DeltaSeconds :type Float%20%28single-precision%29)))

(fn ConstructionScript)